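; Player controller for the tower defense game that owns the UI and relays player actions to BP_ThirdPersonGameMode.
; It creates and updates HUD, lobby, pause, defeat and class-choice widgets, opening class choice on BeginPlay in TD_Game.
; Events forward player, enemy, tower, crate and item requests to the game mode, with F/G/H keys spawning enemies.
; Banker and Builder pawns receive tower and item results, and TransitionMap runs servertravel.
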(event `InputAction|EchapMenu`
  (params (Key :type "Key Structure"))
  ;[1 1 1] Create Pause Menu with Y but it's "EchapMenu"  basic
)

(event `Key|Y`
  (params (Key :type "Key Structure"))
  ;[1 1 1] Create Pause Menu with Y but it's "EchapMenu"  basic
  (:`Pressed`
    (bind _returnvalue (`GameplayStatics.GetCurrentLevelName` true))
    (if (`KismetStringLibrary.EqualEqual_StrStr` _returnvalue "TD_Game")
      (`self.CreateEchapMenu`))))

(event `UpdateUIInfoBase`
  (params (Percent :type "Float (double-precision)"))
  ;[1 1 1] Update UI
  (bind _isvalid_ (`self.CheckTheReferenceLifeBarBase`))
  (if _isvalid_
    (`ProgressBar.SetPercent` (`/Game/Widgets/GameMenu/Base/WBP_InfoBase.BarLife` (`self.WBP_InfoBase_Ref`)) Percent)))

(event `CreateEchapMenu`
  ;[0.1481 0.8297 1] Create Escape Menu
  (bind _returnvalue (`|CreateWidget` "/Game/Widgets/GameMenu/WBP_EchapMenu.WBP_EchapMenu_C"))
  (bind _output_get (set `self.WBP_EchapMenu_Reference` _returnvalue))
  (`UserWidget.AddToViewport` _output_get 0)
  (`WidgetBlueprintLibrary.SetInputMode_UIOnlyEx` self null)
  (set `self.bShowMouseCursor` true))

(event `UpdateUINumberEnemies`
  (params (txt :type Text))
  ;[1 1 1] Update UI
  (bind _isvalid_ (`self.CheckTheReferenceRoundInformations`))
  (if _isvalid_
    (`TextBlock.SetText` (`/Game/Widgets/GameMenu/Round/WBP_Round.Enemies_Txt` (`self.WBP_Round_Ref`)) txt)))

(event `CreateLifeBarBase`
  ;[0.1481 0.8297 1] Create Life Bar Base
  (bind _returnvalue (`|CreateWidget` "/Game/Widgets/GameMenu/Base/WBP_InfoBase.WBP_InfoBase_C"))
  (bind _output_get (set `self.WBP_InfoBase_Ref` _returnvalue))
  (`UserWidget.AddToViewport` _output_get 0))

(event `CreateWidgetFPS`
  ;[0.1481 0.8297 1] CreateWidgetFPS
  (bind _returnvalue (`|CreateWidget` "/Game/Widgets/GameMenu/WBP_FPS.WBP_FPS_C"))
  (`UserWidget.AddToViewport` _returnvalue 0))

(event `UpdateUIRound`
  (params (txt :type Text))
  ;[1 1 1] Update UI
  (bind _isvalid_ (`self.CheckTheReferenceRoundInformations`))
  (if _isvalid_
    (`TextBlock.SetText` (`/Game/Widgets/GameMenu/Round/WBP_Round.Round_txt` (`self.WBP_Round_Ref`)) txt)))

(event `CreateLobby`
  ;[0.1481 0.8297 1] CreateLobby
  (bind _returnvalue (`|CreateWidget` "/Game/Widgets/Lobby/WBP_Lobby.WBP_Lobby_C"))
  (bind _output_get (set `self.WBP_Lobby_Ref` _returnvalue))
  (`UserWidget.AddToViewport` _output_get 0))

(event `CreateWidgetRound`
  ;[0.1481 0.8297 1] Widget Round
  (bind _returnvalue (`|CreateWidget` "/Game/Widgets/GameMenu/Round/WBP_Round.WBP_Round_C"))
  (bind _output_get (set `self.WBP_Round_Ref` _returnvalue))
  (`UserWidget.AddToViewport` _output_get 0))

(event `CreateDefeatWidget`
  ;[0.1481 0.8297 1] Create Defeat Widget
  (bind _returnvalue (`|CreateWidget` "/Game/Widgets/GameMenu/Defeat/WBP_Defeat.WBP_Defeat_C"))
  (bind _output_get (set `self.WBP_Defeated_Ref` _returnvalue))
  (`UserWidget.AddToViewport` _output_get 0)
  (`WidgetBlueprintLibrary.SetInputMode_UIOnlyEx` self null)
  (set `self.bShowMouseCursor` true))

(event `UpdateUILobbyPlayers`
  (params (Txt :type Text))
  ;[1 1 1] Update UI
  (bind _isvalid_ (`self.CheckTheReferenceLobby`))
  (if _isvalid_
    (`TextBlock.SetText` (`/Game/Widgets/Lobby/WBP_Lobby.Players_txt` (`self.WBP_Lobby_Ref`)) Txt)))

(event `CreateTimerLobby`
  ;[0.1481 0.8297 1] CreateTimerLobby
  (bind _returnvalue (`|CreateWidget` "/Game/Widgets/Lobby/WBP_Timer.WBP_Timer_C"))
  (`UserWidget.AddToViewport` _returnvalue 0))

(event `ChooseClass`
  (bind _returnvalue (`|CreateWidget` "/Game/Widgets/MainMenu/WBP_ChooseClass.WBP_ChooseClass_C" self))
  (`UserWidget.AddToViewport` _returnvalue 0)
  (`WidgetBlueprintLibrary.SetInputMode_UIOnlyEx` self null))

(event `SpawnSpeed`
  ;[1 1 1] Spawn Ennemies
  (bind _asbp_third_person_game_mode (cast `/Game/Blueprints/Blueprints/Utilities/BP_ThirdPersonGameMode` (`GameplayStatics.GetGameMode`)))
  (`/Game/Blueprints/Blueprints/Utilities/BP_ThirdPersonGameMode.Spawn Speed` _asbp_third_person_game_mode))

(event `Spawn Basic`
  ;[1 1 1] Spawn Ennemies
  (bind _asbp_third_person_game_mode (cast `/Game/Blueprints/Blueprints/Utilities/BP_ThirdPersonGameMode` (`GameplayStatics.GetGameMode`)))
  (`/Game/Blueprints/Blueprints/Utilities/BP_ThirdPersonGameMode.Spawn Basic` _asbp_third_person_game_mode))

(event `self.ReceiveBeginPlay`
  ;[1 1 1] BeginPlay
  (`self.CreateWidgetFPS`)
  (bind _returnvalue (`GameplayStatics.GetCurrentLevelName` true))
  (if (`KismetStringLibrary.EqualEqual_StrStr` _returnvalue "TD_Game")
    (if (`self.IsLocalPlayerController`)
      (`self.ChooseClass`))))

(event `Spawn Tank`
  ;[1 1 1] Spawn Ennemies
  (bind _asbp_third_person_game_mode (cast `/Game/Blueprints/Blueprints/Utilities/BP_ThirdPersonGameMode` (`GameplayStatics.GetGameMode`)))
  (`/Game/Blueprints/Blueprints/Utilities/BP_ThirdPersonGameMode.Spawn Tank` _asbp_third_person_game_mode))

(event `TransitionMap`
  (params (NameMap :type String))
  ;[1 1 1] Transition Map
  (`KismetSystemLibrary.ExecuteConsoleCommand` (`KismetStringLibrary.Concat_StrStr` "servertravel " NameMap) null))

(event `Key|F`
  (params (Key :type "Key Structure"))
  ;[1 1 1] Spawn Ennemies
  (:`Pressed`
    (`self.SpawnSpeed`)))

(event `Key|G`
  (params (Key :type "Key Structure"))
  ;[1 1 1] Spawn Ennemies
  (:`Pressed`
    (`self.Spawn Basic`)))

(event `Key|H`
  (params (Key :type "Key Structure"))
  ;[1 1 1] Spawn Ennemies
  (:`Pressed`
    (`self.Spawn Tank`)))

(event `CreatePlayer_Server`
  (params (`isBanker?` :type Boolean))
  (bind _asbp_third_person_game_mode (cast `/Game/Blueprints/Blueprints/Utilities/BP_ThirdPersonGameMode` (`GameplayStatics.GetGameMode`)))
  (`/Game/Blueprints/Blueprints/Utilities/BP_ThirdPersonGameMode.Spawn Player` _asbp_third_person_game_mode self `isBanker?`))

(event `SpawnTower`
  (params (TowerClass :type "/Game/Blueprints/Blueprints/Tower/BP_Tower Class Reference") (Location :type "Vector Structure") (PlayerIndex :type Integer))
  ;[1 1 1] Spawn Tower
  (bind _asbp_third_person_game_mode (cast `/Game/Blueprints/Blueprints/Utilities/BP_ThirdPersonGameMode` (`GameplayStatics.GetGameMode`)))
  (bind _spawnedtower (`/Game/Blueprints/Blueprints/Utilities/BP_ThirdPersonGameMode.SpawnTower` _asbp_third_person_game_mode TowerClass Location))
  (bind _asbp_banker (cast `/Game/Blueprints/Blueprints/Characters/BP_Banker` (`GameplayStatics.GetPlayerPawn` PlayerIndex)))
  (set `/Game/Blueprints/Blueprints/Characters/BP_Banker.currentMovingTower` _spawnedtower _asbp_banker))

(event `SpawnCrate`
  (params (Location :type "Vector Structure") (TypeClass :type "/Game/Blueprints/Blueprints/Item/BP_Crate Class Reference"))
  ;[1 0 0] SpawnCrate
  (bind _asbp_third_person_game_mode (cast `/Game/Blueprints/Blueprints/Utilities/BP_ThirdPersonGameMode` (`GameplayStatics.GetGameMode`)))
  (`/Game/Blueprints/Blueprints/Utilities/BP_ThirdPersonGameMode.SpawnCrate` _asbp_third_person_game_mode TypeClass Location))

(event `DestroyTower`
  (params (PlayerIndex :type Integer))
  ;[1 1 1] Destroy Tower
  (`|ExecutionSequence`
    (:`then_0`
      (bind _asbp_banker (cast `/Game/Blueprints/Blueprints/Characters/BP_Banker` (`GameplayStatics.GetPlayerPawn` PlayerIndex))))
    (:`then_1`
      (bind _asbp_third_person_game_mode (cast `/Game/Blueprints/Blueprints/Utilities/BP_ThirdPersonGameMode` (`GameplayStatics.GetGameMode`)))
      (`/Game/Blueprints/Blueprints/Utilities/BP_ThirdPersonGameMode.Destroy ActorServer` _asbp_third_person_game_mode (`/Game/Blueprints/Blueprints/Characters/BP_Banker.currentMovingTower` _asbp_banker))
      (set `/Game/Blueprints/Blueprints/Characters/BP_Banker.currentMovingTower` null _asbp_banker))))

(event `Destroy Crate`
  (params (Crate :type "/Game/Blueprints/Blueprints/Item/BP_Crate Object Reference"))
  ;[1 0 0] DestroyCrate
  (bind _asbp_third_person_game_mode (cast `/Game/Blueprints/Blueprints/Utilities/BP_ThirdPersonGameMode` (`GameplayStatics.GetGameMode`)))
  (`/Game/Blueprints/Blueprints/Utilities/BP_ThirdPersonGameMode.Destroy Actor Server` _asbp_third_person_game_mode Crate))

(event `PlaceTower`
  (params (Tower :type "/Game/Blueprints/Blueprints/Tower/BP_Tower Object Reference"))
  ;[1 1 1] Place Tower
  (set `/Game/Blueprints/Blueprints/Tower/BP_Tower.isPlaced?` true Tower)
  (`/Game/Blueprints/Blueprints/Tower/BP_Tower.PlaceTower` Tower))

(event `MoveActor`
  (params (`Tower Actor` :type "Actor Object Reference") (Location :type "Vector Structure"))
  (`self.K2_SetActorLocation` `Tower Actor` Location false false))

(event `AddItemBuilder`
  (params (Inventory :type "/Game/Structs/S_BuilderInventory Structure") (Crate :type "/Game/Blueprints/Blueprints/Item/BP_Crate Object Reference") (Player :type "/Game/Blueprints/Blueprints/Characters/BP_Player Object Reference"))
  ;[1 0 0] Add Consumable to the Builder
  (bind _asbp_third_person_game_mode (cast `/Game/Blueprints/Blueprints/Utilities/BP_ThirdPersonGameMode` (`GameplayStatics.GetGameMode`)))
  (`/Game/Blueprints/Blueprints/Utilities/BP_ThirdPersonGameMode.AddBuilderItem` _asbp_third_person_game_mode Inventory Crate Player))

(event `TowerProceduralAnimation`
  (params (Tower :type "/Game/Blueprints/Blueprints/Tower/BP_Tower Object Reference"))
  (`/Game/Blueprints/Blueprints/Tower/BP_Tower.ProceduralAnimation` Tower))

(event `Spawn Item`
  (params (Location :type "Vector Structure") (Class :type "Actor Class Reference") (ControlledPawn :type "Actor Object Reference"))
  ;[1 0 0] SpawnItem
  (bind _asbp_third_person_game_mode (cast `/Game/Blueprints/Blueprints/Utilities/BP_ThirdPersonGameMode` (`GameplayStatics.GetGameMode`)))
  (`/Game/Blueprints/Blueprints/Utilities/BP_ThirdPersonGameMode.Spawn Item` _asbp_third_person_game_mode Location Class ControlledPawn))

(event `MoveItem`
  (params (Actor :type "Actor Object Reference") (Location :type "Vector Structure") (Rotator :type "Rotator Structure"))
  ;[1 0 0] MoveItem
  (bind _asbp_third_person_game_mode (cast `/Game/Blueprints/Blueprints/Utilities/BP_ThirdPersonGameMode` (`GameplayStatics.GetGameMode`)))
  (`/Game/Blueprints/Blueprints/Utilities/BP_ThirdPersonGameMode.Move Actor` _asbp_third_person_game_mode Actor Location Rotator))

(event `GetItemOnMap`
  ;[1 0 0] Get Item On Map
  (bind _asbp_third_person_game_mode (cast `/Game/Blueprints/Blueprints/Utilities/BP_ThirdPersonGameMode` (`GameplayStatics.GetGameMode`)))
  (bind _asbp_builder (cast `/Game/Blueprints/Blueprints/Characters/BP_Builder` (`self.K2_GetPawn`)))
  (`/Game/Blueprints/Blueprints/Utilities/BP_ThirdPersonGameMode.Get All Item Class Server` _asbp_third_person_game_mode _asbp_builder))

(event `DestroyItemServer`
  (params (Actor :type "Actor Object Reference"))
  ;[1 0 0] Destroy Item in the server
  (bind _asbp_third_person_game_mode (cast `/Game/Blueprints/Blueprints/Utilities/BP_ThirdPersonGameMode` (`GameplayStatics.GetGameMode`)))
  (`/Game/Blueprints/Blueprints/Utilities/BP_ThirdPersonGameMode.Destroy Actor Server` _asbp_third_person_game_mode Actor))

(fn `CheckTheReferenceLifeBarBase`
  (returns (`isValid?` :type Boolean))
  (`/Engine/EditorBlueprintResources/StandardMacros.IsValid` (`self.WBP_InfoBase_Ref`)
    (:`Is Valid`
      (return true))
    (:`Is Not Valid`
      (bind _foundwidgets (`WidgetBlueprintLibrary.GetAllWidgetsOfClass` "/Game/Widgets/GameMenu/Base/WBP_InfoBase.WBP_InfoBase_C" false))
      (set `self.WBP_InfoBase_Ref` (`|GetArrayItem` _foundwidgets))
      (return false))))

(fn `CheckTheReferenceLobby`
  (returns (`isValid?` :type Boolean))
  (`/Engine/EditorBlueprintResources/StandardMacros.IsValid` (`self.WBP_Lobby_Ref`)
    (:`Is Valid`
      (return true))
    (:`Is Not Valid`
      (bind _foundwidgets (`WidgetBlueprintLibrary.GetAllWidgetsOfClass` "/Game/Widgets/Lobby/WBP_Lobby.WBP_Lobby_C" false))
      (set `self.WBP_Lobby_Ref` (`|GetArrayItem` _foundwidgets))
      (return false))))

(fn `CheckTheReferenceRoundInformations`
  (returns (`isValid?` :type Boolean))
  (`/Engine/EditorBlueprintResources/StandardMacros.IsValid` (`self.WBP_Round_Ref`)
    (:`Is Valid`
      (return true))
    (:`Is Not Valid`
      (bind _foundwidgets (`WidgetBlueprintLibrary.GetAllWidgetsOfClass` "/Game/Widgets/GameMenu/Round/WBP_Round.WBP_Round_C" false))
      (set `self.WBP_Round_Ref` (`|GetArrayItem` _foundwidgets))
      (return false))))

(fn `UserConstructionScript`)