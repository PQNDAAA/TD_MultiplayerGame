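; BP_Unit is a damageable base whose destruction triggers game over.
; AnyDamage feeds TakeDamage, which subtracts from SUnitInfo.Health while it is above zero, after which UpdateUI sends the health ratio to BP_ThirdPersonGameMode.
; Health is checked before subtraction, so only a hit arriving at zero or below destroys the actor and calls the game mode's DestroyGameOver through BaseDead.
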(event `UpdateUI`
  (bind (_name _damage _health _defense _speed _maxhealth) (break `/Game/Structs/S_Unit` (`self.S_UnitInfo`)))
  ;[1 0 0] Update UI Base
  (bind _asbp_third_person_game_mode (cast `/Game/Blueprints/Blueprints/Utilities/BP_ThirdPersonGameMode` (`GameplayStatics.GetGameMode`)))
  (`/Game/Blueprints/Blueprints/Utilities/BP_ThirdPersonGameMode.UIBaseAll` _asbp_third_person_game_mode (/ _health _maxhealth)))

(event `BaseDead`
  ;[1 0 0] Game Over
  (bind _asbp_third_person_game_mode (cast `/Game/Blueprints/Blueprints/Utilities/BP_ThirdPersonGameMode` (`GameplayStatics.GetGameMode`)))
  (`/Game/Blueprints/Blueprints/Utilities/BP_ThirdPersonGameMode.Destroy Game Over` _asbp_third_person_game_mode))

(event `self.ReceiveAnyDamage`
  (params (Damage :type "Float (single-precision)") (DamageType :type "DamageType Object Reference") (InstigatedBy :type "Controller Object Reference") (DamageCauser :type "Actor Object Reference"))
  ;[1 1 1] Take Damage
  (bind _isdead_ (`self.TakeDamage` Damage self))
  (if (== _isdead_ false)
    ;[1 1 1] Update after damage
    (`self.UpdateUI`)
    (else
      ;[1 1 1] Event GameOver
      (`self.BaseDead`))))

(fn `TakeDamage`
  (params (Damage :type "Float (double-precision)") (Actor :type "Actor Object Reference"))
  (returns (`IsDead?` :type Boolean))
  (locals (isDead :type Boolean))
  (bind (_name _damage _health) (break `/Game/Structs/S_Unit` (`self.S_UnitInfo`)))
  ;[1 1 1] The base takes damage and the function checks if he is always here ( > 0 )
  (if (> _health 0.0)
    (set `self.FinalHealth` (- _health Damage))
    (`|VariableSetRef` (`.Health_11_2727ED6C4B492BC37991F5AD08FE0B56` (break `/Game/Structs/S_Unit` (`self.S_UnitInfo`))) (`self.FinalHealth`))
    (return false)
    (else
      (bind _output_get (set `local.isDead` true))
      (`self.K2_DestroyActor` Actor)
      (return _output_get))))

(fn `UserConstructionScript`)