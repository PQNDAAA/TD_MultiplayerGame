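; Troop AI character that advances on the first BP_Base_2 actor and attacks what it overlaps.
; On BeginPlay it loads its DT_Troops row by name, scales combat stats by the game mode's round number, and fills its info widget.
; Tick reissues AI MoveTo every frame; overlap starts a delayed gate loop applying damage.
; Incoming damage runs through TakeDamage with defense; the damage-popup logic is unconnected.
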(event `UpdateUAll`
  ;[1 1 1] Update UI All
  (bind _aswbp_troops_info (cast `/Game/Widgets/GameMenu/Troops/WBP_TroopsInfo` (`WidgetComponent.GetUserWidgetObject` (`self.Widget`))))
  (`ProgressBar.SetPercent` (`/Game/Widgets/GameMenu/Troops/WBP_TroopsInfo.BarLife` _aswbp_troops_info) (/ (`self.Health`) (`self.MaxHealth`)))
  (`TextBlock.SetText` (`/Game/Widgets/GameMenu/Troops/WBP_TroopsInfo.TroopsName` _aswbp_troops_info) (`KismetTextLibrary.Conv_StringToText` (`KismetStringLibrary.Conv_NameToString` (`self.Name`)))))

(event `self.ReceiveBeginPlay`
  ;[1 1 1] Calculate Stats at the Beginning
  (`self.CalculateStats`)
  ;[1 1 1] Set Speed At The Beginning
  (`self.SetSpeed` (`self.Speed`))
  ;[1 1 1] Update UI at the beginning
  (`self.UpdateUAll`)
  (`SceneComponent.SetVisibility` (`self.WidgetDamageFeedback`) false false))

(event `self.ReceiveTick`
  (params (DeltaSeconds :type "Float (single-precision)"))
  ;[1 1 1] Move To The Base
  (`/Engine/EditorBlueprintResources/ActorMacros.Switch Has Authority`
    (:`Authority`
      _)
    (:`Remote`
      _))
  (`self.MoveTo`))

(event `self.ReceiveActorBeginOverlap`
  (params (OtherActor :type "Actor Object Reference"))
  ;[1 1 1] Loop Damage when Collide
  (if (!= OtherActor self)
    (`|ExecutionSequence`
      (:`then_0`
        (goto _label :!via `Open`))
      (:`then_1`
        (`/Engine/EditorBlueprintResources/StandardMacros.Gate` true :!label _label
          (:`Exit`
            (`GameplayStatics.ApplyDamage` OtherActor (`self.Damage`) null self)
            (`KismetSystemLibrary.Delay` (`self.AttackSpeed`))
            (goto _label)))))))

(event `MoveTo`
  ;[1 1 1] Event MoveTo Base
  (`/Engine/EditorBlueprintResources/ActorMacros.Switch Has Authority`
    (:`Authority`
      _)
    (:`Remote`
      _))
  (`|AIMoveTo` self (0.0 0.0 0.0) (`self.GetBaseActor`) 0.0))

(event `self.ReceiveAnyDamage`
  (params (Damage :type "Float (single-precision)") (DamageType :type "DamageType Object Reference") (InstigatedBy :type "Controller Object Reference") (DamageCauser :type "Actor Object Reference"))
  ;[1 1 1] Take Damage
  (bind (_final_health _isdead_) (`self.TakeDamage` Damage (`self.Health`) (`self.Defense`) self))
  (if (== _isdead_ false)
    (set `self.Health` _final_health)
    ;[1 1 1] Update after damage
    (`self.UpdateUAll`)))

(fn `CalculateStats`
  (bind _asbp_third_person_game_mode (cast `/Game/Blueprints/Blueprints/Utilities/BP_ThirdPersonGameMode` (`GameplayStatics.GetGameMode`)))
  ;[1 1 1] Get the troops datable
  (bind _returnvalue (`|GetDataTableRow` "/Game/Datatables/DT_Troops.DT_Troops" (`self.Name`))
    (:`then`
      (bind (_name _damage _health _defense _speed _maxhealth _attackspeed) (break `/Game/Structs/S_Unit` _returnvalue))
      (bind _numberround (`/Game/Blueprints/Blueprints/Utilities/BP_ThirdPersonGameMode.NumberRound` _asbp_third_person_game_mode))
      ;[1 1 1] Set different variables
      (set `self.Health` (* _health _numberround))
      (set `self.Damage` (+ _damage _numberround))
      (set `self.Defense` (+ (* _defense 1.1) _numberround))
      (set `self.Speed` _speed)
      (set `self.MaxHealth` (* _maxhealth _numberround))
      (set `self.AttackSpeed` _attackspeed))))

(fn `GetBaseActor`
  (returns (`Base Actor` :type "Actor Object Reference"))
  (bind _outactors (`GameplayStatics.GetAllActorsOfClass` "/Game/Blueprints/Blueprints/Base/BP_Base_2.BP_Base_2_C"))
  (return (`|GetArrayItem` _outactors)))

(fn `UserConstructionScript`)