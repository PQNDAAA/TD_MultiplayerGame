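; BP_Entity is a character Blueprint with shared damage, death payout and walk-speed logic for troops.
; TakeDamage returns health reduced by defense-scaled damage, treating the target as dead only when the incoming health is already zero or below.
; On death it calls AddBankerMoney, which finds BP_Banker entries in the game mode's Players and adds MoneyDrop to their controlled pawns, then destroys the target actor.
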(event Custom|AddBankerMoney
  ;[1 0.1042 0.1042] Give Money To banker on death
  (bind _asbp_third_person_game_mode (Utilities|Casting|CastToBP_ThirdPersonGameMode (Game|GetGameMode)))
  (bind (_array_element _array_index) (Utilities|Array|ForEachLoopwithBreak (Variables|/Game/Blueprints/Blueprints/Utilities/BP_ThirdPersonGameMode.BP_ThirdPersonGameMode_C|GetPlayers _asbp_third_person_game_mode))
    (:LoopBody
      (if (== (Utilities|GetClass _array_element) "/Game/Blueprints/Blueprints/Characters/BP_Banker.BP_Banker_C")
        (bind _asbp_banker (Utilities|Casting|CastToBP_Banker (Pawn|GetControlledPawn (Game|GetPlayerController _array_index))))
        (Default|AddMoney _asbp_banker (Variables|Default|GetmoneyDrop))))))

(fn ConstructionScript)

(fn TakeDamage
  (params (Damage :type Float%20%28double-precision%29) (Health :type Float%20%28double-precision%29) (Defense :type Float%20%28double-precision%29) (ActorTarget :type Actor%20Object%20Reference))
  ;[1 1 1] This function calculates the damage that the person will take and checks the life
  (if (> Health 0.0)
    (bind _output_get (LocalVariables|SetFinalDamage (|(attack*(100/(100+defense))) Damage Defense)))
    (bind _output_get_2 (LocalVariables|SetFinalHealth (- Health _output_get)))
    (return _output_get_2 false)
    (else
      (bind _output_get_3 (LocalVariables|SetisDead true))
      (CallFunction|AddBankerMoney)
      (Actor|DestroyActor ActorTarget)
      (return 0.0 _output_get_3))))

(fn SetSpeed
  (params (Max%20Walk%20Speed :type Float%20%28double-precision%29))
  ;[1 1 1] Set Speed for the troops
  (Variables|/Script/Engine.CharacterMovementComponent|SetMaxWalkSpeed (Variables|Character|GetCharacterMovement) Max%20Walk%20Speed))