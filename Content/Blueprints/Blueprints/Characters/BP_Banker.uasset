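; Banker player character that flies a zoomable drone camera and spends money to build towers and drop crates.
; The construction script fills tower classes and prices from DT_TowerData; shortcuts in construction mode spawn a tower that a 0.05-second Delay loop moves to the camera's forward trace until placed.
; Crates drop at a cursor trace.
; BP_PlayerController handles spawning, moving, placing and destroying, while the game mode computes money deductions.
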(event `Key|V`
  (params (Key :type "Key Structure"))
  (bind _returnvalue (`GameplayStatics.GetPlayerController` 0))
  (bind (_locationx _locationy) (`PlayerController.GetMousePosition` _returnvalue))
  (bind (_worldposition _worlddirection) (`GameplayStatics.DeprojectScreenToWorld` _returnvalue (`KismetMathLibrary.MakeVector2D` _locationx _locationy)))
  ;[0.04167 0.4576 1] Drop the crate
  (:`Pressed`
    (if (> (`self.Money`) 0)
      (bind _outactors (`GameplayStatics.GetAllActorsOfClass` "/Game/Blueprints/Blueprints/Item/BP_Crate.BP_Crate_C"))
      (bind _outhit (`KismetSystemLibrary.LineTraceSingle` _worldposition (+ _worldposition (* _worlddirection 15000.0)) "TraceTypeQuery1" true _outactors))
      (bind _asbp_player_controller (cast `/Game/Blueprints/Blueprints/Utilities/BP_PlayerController` (`GameplayStatics.GetPlayerController` 0)))
      (if (== (`self.CrateNumber`) 0)
        ;[1 0.1042 0.1042] On server
        (`/Game/Blueprints/Blueprints/Utilities/BP_PlayerController.SpawnCrate` _asbp_player_controller (`.Location` (`GameplayStatics.BreakHitResult` _outhit)) "/Game/Blueprints/Blueprints/Item/BP_CrateBarbedWire.BP_CrateBarbedWire_C")
        (else
          (`/Game/Blueprints/Blueprints/Utilities/BP_PlayerController.SpawnCrate` _asbp_player_controller (`.Location` (`GameplayStatics.BreakHitResult` _outhit)) "/Game/Blueprints/Blueprints/Item/BP_CrateMine.BP_CrateMine_C")))
      (`self.SubstractMoney` 125))))

(event `InputAxis|Move Forward / Backward`
  (params (AxisValue :type "Float (single-precision)"))
  (bind _drone (`self.Drone`))
  ;[0.04167 0.4576 1] Move Camera
  (`SceneComponent.K2_AddWorldOffset` _drone (* (`SceneComponent.GetForwardVector` _drone) (* AxisValue (`self.CameraSpeed`))) false false))

(event `AddBankerUI`
  (bind _returnvalue (`GameplayStatics.GetPlayerController` 0))
  ;[0.04167 0.4576 1] Add UI
  (bind _returnvalue_2 (`|CreateWidget` "/Game/Widgets/GameMenu/Banker/WBP_MainHUDBanker.WBP_MainHUDBanker_C"))
  (set `/Game/Widgets/GameMenu/Banker/WBP_MainHUDBanker.Money` (`self.Money`) _returnvalue_2)
  (`UserWidget.AddToViewport` _returnvalue_2 0)
  (`WidgetBlueprintLibrary.SetInputMode_GameAndUIEx` _returnvalue null "DoNotLock" false)
  (set `PlayerController.bShowMouseCursor` true _returnvalue))

(event `InputAxis|Move Right / Left`
  (params (AxisValue :type "Float (single-precision)"))
  (bind _drone (`self.Drone`))
  ;[0.04167 0.4576 1] Move Camera
  (`SceneComponent.K2_AddWorldOffset` _drone (* (`SceneComponent.GetRightVector` _drone) (* AxisValue (`self.CameraSpeed`))) false false))

(event `Key|MouseScrollUp`
  (params (Key :type "Key Structure"))
  (bind _drone (`self.Drone`))
  (bind (_returnvalue_x _returnvalue_y _returnvalue_z) (`KismetMathLibrary.BreakVector` (`SceneComponent.K2_GetComponentLocation` _drone)))
  ;[0.04167 0.4576 1] Zoom / Dezoom Camera
  (:`Pressed`
    (if (> _returnvalue_z (`self.CameraZoomMax`))
      (`SceneComponent.K2_AddWorldOffset` _drone (* (* (`SceneComponent.GetUpVector` _drone) -1) (`self.CameraZoomSpeed`)) false false))))

(event `InputAction|Shift`
  (params (Key :type "Key Structure"))
  (bind _cameraspeed (`self.CameraSpeed`))
  ;[0.04167 0.4576 1] Increase Camera Speed
  (:`Pressed`
    (set `self.CameraSpeed` (* _cameraspeed 2.5)))
  (:`Released`
    (set `self.CameraSpeed` (/ _cameraspeed 2.5))))

(event `Key|MouseScrollDown`
  (params (Key :type "Key Structure"))
  (bind _drone (`self.Drone`))
  (bind (_returnvalue_x _returnvalue_y _returnvalue_z) (`KismetMathLibrary.BreakVector` (`SceneComponent.K2_GetComponentLocation` _drone)))
  ;[0.04167 0.4576 1] Zoom / Dezoom Camera
  (:`Pressed`
    (if (< _returnvalue_z (`self.CameraZoomMin`))
      (`SceneComponent.K2_AddWorldOffset` _drone (* (`SceneComponent.GetUpVector` _drone) (`self.CameraZoomSpeed`)) false false))))

(event `Key|LeftMouseButton`
  (params (Key :type "Key Structure"))
  (bind _currentmovingtower (`self.currentMovingTower`))
  (bind _currentmovingtower_2 (`self.currentMovingTower`))
  ;[0.04167 0.4576 1] Check if can place Tower
  (:`Pressed`
    (if (`self.ConstructionMode`)
      (`/Engine/EditorBlueprintResources/StandardMacros.IsValid` _currentmovingtower
        (:`Is Valid`
          (if (`/Game/Blueprints/Blueprints/Tower/BP_Tower.CanBePlaced?` _currentmovingtower)
            (set `self.MovingTower` false)
            (bind _asbp_player_controller (cast `/Game/Blueprints/Blueprints/Utilities/BP_PlayerController` (`GameplayStatics.GetPlayerController` 0)))
            ;[1 0.1042 0.1042] Place tower
            (`/Game/Blueprints/Blueprints/Utilities/BP_PlayerController.PlaceTower` _asbp_player_controller _currentmovingtower_2)
            (`self.SubstractMoney` (`|GetArrayItem` (`self.ConstructionTowerPrice`) (`self.ConstructionTowerSelection`)))
            (`/Game/Blueprints/Blueprints/Tower/BP_Tower.GetEnemy` _currentmovingtower_2)
            (set `self.currentMovingTower` null)))))))

(event `InputAction|Jump`
  (params (Key :type "Key Structure"))
  ;[1 0.1042 0.1042] Enable Construction Mode
  (:`Pressed`
    (`/Engine/EditorBlueprintResources/StandardMacros.FlipFlop`
      (:`A`
        (set `self.ConstructionMode` true))
      (:`B`
        (`self.Change Moving Tower`)
        (set `self.ConstructionMode` false)
        (set `self.TowerSelected?` false)
        (set `self.ConstructionTowerSelection` -1)))))

(event `Spawn&Move tower`
  (bind _returnvalue (`GameplayStatics.GetPlayerController` 0))
  (if (>= (`self.Money`) (`|GetArrayItem` (`self.ConstructionTowerPrice`) (`self.ConstructionTowerSelection`)))
    ;[1 0.1042 0.1042] SpawnTower
    (bind _asbp_player_controller (cast `/Game/Blueprints/Blueprints/Utilities/BP_PlayerController` _returnvalue))
    (`/Game/Blueprints/Blueprints/Utilities/BP_PlayerController.SpawnTower` _asbp_player_controller (`|GetArrayItem` (`self.ConstructionTowerClass`) (`self.ConstructionTowerSelection`)) (0.0 0.0 0.0) (`self.playerIndex`))
    (set `self.MovingTower` true)
    ;[1 0.1042 0.1042] MoveTower
    (`KismetSystemLibrary.Delay` 0.05 :!label _label)
    (if (`self.ConstructionMode`)
      (if (`self.MovingTower`)
        (bind _location (`self.ForwardRaycast`))
        (bind _asbp_player_controller_2 (cast `/Game/Blueprints/Blueprints/Utilities/BP_PlayerController` _returnvalue))
        (`/Game/Blueprints/Blueprints/Utilities/BP_PlayerController.MoveActor` _asbp_player_controller_2 (`self.currentMovingTower`) (`KismetMathLibrary.MakeVector` (.x _location) (.y _location)))
        (goto _label)))))

(event `InputAction|Shortcut0`
  (params (Key :type "Key Structure"))
  ;[1 0.1042 0.1042] Change MovingTower
  (:`Pressed`
    (if (`self.ConstructionMode`)
      (set `self.TowerSelected?` true)
      (`self.Change Moving Tower`)
      (set `self.ConstructionTowerSelection` 0)
      (`self.Spawn&Move tower` :!label _label_2))))

(event `InputAction|Shortcut1`
  (params (Key :type "Key Structure"))
  ;[1 0.1042 0.1042] Change MovingTower
  (:`Pressed`
    (if (`self.ConstructionMode`)
      (set `self.TowerSelected?` true)
      (`self.Change Moving Tower`)
      (set `self.ConstructionTowerSelection` 1)
      (goto _label_2))))

(event `SubstractMoney`
  (params (moneysubstact :type Integer))
  ;[1 0 0] Substract Money
  (bind _asbp_third_person_game_mode (cast `/Game/Blueprints/Blueprints/Utilities/BP_ThirdPersonGameMode` (`GameplayStatics.GetGameMode`)))
  (bind _newmoney (`/Game/Blueprints/Blueprints/Utilities/BP_ThirdPersonGameMode.SubstractMoney` _asbp_third_person_game_mode (`self.Money`) moneysubstact))
  (set `self.Money` _newmoney))

(fn `AddMoney`
  (params (Amount :type Integer))
  (set `self.Money` (+ (`self.Money`) Amount)))

(fn `Change Moving Tower`
  (if (`self.ConstructionMode`)
    (if (`self.MovingTower`)
      (set `self.MovingTower` false)
      (bind _asbp_player_controller (cast `/Game/Blueprints/Blueprints/Utilities/BP_PlayerController` (`GameplayStatics.GetPlayerController` 0)))
      (`/Game/Blueprints/Blueprints/Utilities/BP_PlayerController.DestroyTower` _asbp_player_controller (`self.playerIndex`)))
    (return)))

(fn `ForwardRaycast`
  (returns (Location :type "Vector Structure"))
  (bind _camera (`self.Camera`))
  (bind _returnvalue (`SceneComponent.K2_GetComponentLocation` _camera))
  (bind _outhit (`KismetSystemLibrary.LineTraceSingle` _returnvalue (+ _returnvalue (* (`KismetMathLibrary.GetForwardVector` (`SceneComponent.K2_GetComponentRotation` _camera)) 15000.0)) "TraceTypeQuery1"))
  (return (`.Location` (`GameplayStatics.BreakHitResult` _outhit))))

(fn `UserConstructionScript`
  (bind _constructiontowerclass (`self.ConstructionTowerClass`))
  (bind _outrownames (`DataTableFunctionLibrary.GetDataTableRowNames` "/Game/Datatables/DT_TowerData.DT_TowerData"))
  (for _array_element _outrownames
    (bind _returnvalue (`|GetDataTableRow` "/Game/Datatables/DT_TowerData.DT_TowerData" _array_element)
      (:`then`
        (if (not (`KismetArrayLibrary.Array_Contains` _constructiontowerclass (`.Class_29_4D81F8344673072C65A1A39E500251F5` (break `/Game/Structs/S_TowerData` _returnvalue))))
          (`KismetArrayLibrary.Array_AddUnique` (`self.ConstructionTowerPrice`) (break `/Game/Structs/S_TowerData` _returnvalue))
          (`KismetArrayLibrary.Array_AddUnique` _constructiontowerclass (`.Class_29_4D81F8344673072C65A1A39E500251F5` (break `/Game/Structs/S_TowerData` _returnvalue)))
          (`parent.UserConstructionScript`))))))