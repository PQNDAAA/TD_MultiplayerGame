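; BP_Mine is a mine item that damages troop characters who walk onto it.
; On overlap with a BP_TroopsCharacter it applies its damage to that actor and destroys itself.
; Its construction script scales damage linearly with the round number read from BP_ThirdPersonGameMode, so mines created in later rounds hit harder.
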(event `self.ReceiveActorBeginOverlap`
  (params (OtherActor :type "Actor Object Reference"))
  ;[1 1 1] Take damage
  (cast `/Game/Blueprints/Blueprints/AI/Troops/BP_TroopsCharacter` OtherActor)
  (`GameplayStatics.ApplyDamage` OtherActor (`self.Damage`))
  (`self.K2_DestroyActor`))

(fn `UserConstructionScript`
  ;[1 1 1] Increase the Mine damages each round
  (bind _asbp_third_person_game_mode (cast `/Game/Blueprints/Blueprints/Utilities/BP_ThirdPersonGameMode` (`GameplayStatics.GetGameMode`)))
  (set `self.Damage` (`KismetMathLibrary.Conv_IntToDouble` (* 200 (`/Game/Blueprints/Blueprints/Utilities/BP_ThirdPersonGameMode.NumberRound` _asbp_third_person_game_mode)))))