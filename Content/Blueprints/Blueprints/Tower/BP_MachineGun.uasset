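; BP_MachineGun is a machine gun tower Blueprint that turns to face its first target.
; Its ProceduralAnimation override computes a look-at yaw to Target[0], adds a 90-degree offset and writes it to TowerZRotation on the BasicTower1 mesh's ABP_Sentinelle anim instance.
; The parent implementation runs afterward, only when the target and cast are valid.
; All other logic is inherited, as the event graph is empty.
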(fn `ProceduralAnimation`
  (bind _output (`|GetArrayItem` (`self.Target`)))
  (bind (_returnvalue_roll _returnvalue_pitch _returnvalue_yaw) (`KismetMathLibrary.BreakRotator` (`KismetMathLibrary.FindLookAtRotation` (`self.K2_GetActorLocation` self) (`self.K2_GetActorLocation` _output))))
  (`/Engine/EditorBlueprintResources/StandardMacros.IsValid` _output
    (:`Is Valid`
      (bind _asabp_sentinelle (cast `/Game/Animation/ABP_Sentinelle` (`SkeletalMeshComponent.GetAnimInstance` (`self.basicTower1`))))
      (set `/Game/Animation/ABP_Sentinelle.TowerZRotation` (+ _returnvalue_yaw 90.0) _asabp_sentinelle)
      (`parent.ProceduralAnimation`))))

(fn `UserConstructionScript`
  (`parent.UserConstructionScript`))