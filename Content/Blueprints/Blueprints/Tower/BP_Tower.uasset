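; Tower actor for a tower-defense game that can be placed and damages troop characters entering its range sphere.
; Construction loads damage, fire interval and range from DT_TowerData by name and level.
; Before placement, HitBox overlaps toggle validity and a red material; PlaceTower switches collision profiles.
; Once placed, a delay-driven loop damages the first tracked target and triggers procedural animation through player controllers.
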(event `self.ShootingRangeHibox.OnComponentBeginOverlap`
  (params (OverlappedComponent :type "PrimitiveComponent Object Reference") (OtherActor :type "Actor Object Reference") (OtherComp :type "PrimitiveComponent Object Reference") (OtherBodyIndex :type Integer) (bFromSweep :type Boolean) (SweepResult :type "HitResult Structure (by ref)"))
  ;[1 1 1] Attack on actor enter sphere collider
  (if (`self.isPlaced?`)
    (bind _asbp_troops_character (cast `/Game/Blueprints/Blueprints/AI/Troops/BP_TroopsCharacter` OtherActor))
    (`KismetArrayLibrary.Array_AddUnique` (`self.Target`) _asbp_troops_character)
    (`self.Attack`)))

(event `self.ShootingRangeHibox.OnComponentEndOverlap`
  (params (OverlappedComponent :type "PrimitiveComponent Object Reference") (OtherActor :type "Actor Object Reference") (OtherComp :type "PrimitiveComponent Object Reference") (OtherBodyIndex :type Integer))
  (bind _target (`self.Target`))
  ;[1 1 1] Remove out enemy
  (if (`self.isPlaced?`)
    (bind _asbp_troops_character (cast `/Game/Blueprints/Blueprints/AI/Troops/BP_TroopsCharacter` OtherActor))
    (if (`KismetArrayLibrary.Array_Contains` _target _asbp_troops_character)
      (`KismetArrayLibrary.Array_RemoveItem` _target _asbp_troops_character))))

(event `Attack`
  (if (not (`self.isAttacking?`))
    (set `self.isAttacking?` true)
    (if (`KismetArrayLibrary.Array_IsNotEmpty` (`self.Target`)) :!label _label
      (`|ExecutionSequence`
        (:`then_0`
          ;[1 0.1042 0.1042] Damage
          (`KismetSystemLibrary.Delay` (`self.AttackSpeed`))
          (`GameplayStatics.ApplyDamage` (`|GetArrayItem` (`self.Target`)) (`self.AttackDamage`)))
        (:`then_1`
          ;[0.04167 0.4576 1] Procedural Animation
          (bind _asbp_third_person_game_mode (cast `/Game/Blueprints/Blueprints/Utilities/BP_ThirdPersonGameMode` (`GameplayStatics.GetGameMode`)))
          (for _array_element (`/Game/Blueprints/Blueprints/Utilities/BP_ThirdPersonGameMode.Players` _asbp_third_person_game_mode)
            (bind _asbp_player_controller (cast `/Game/Blueprints/Blueprints/Utilities/BP_PlayerController` (`self.GetController` _array_element)))
            (`/Game/Blueprints/Blueprints/Utilities/BP_PlayerController.TowerProceduralAnimation` _asbp_player_controller self)
            (`KismetSystemLibrary.Delay` 0.001)
            (goto _label))))
      (else
        (set `self.isAttacking?` false)))))

(event `CantBePlaced`
  ;[0.8899 0.6719 1] Can Be placed?
  (if (not (`self.isPlaced?`))
    (`self.SetTowerMaterial` "/Game/Material/MaterialInstance/M_RedAvailableArea.M_RedAvailableArea")
    (set `self.CanBePlaced?` false)))

(event `CanBePlaced`
  ;[0.8899 0.6719 1] Can Be placed?
  (if (not (`self.isPlaced?`))
    (`self.SetTowerMaterial` (`self.BasicMaterial`))
    (set `self.CanBePlaced?` true)))

(event `self.HitBox.OnComponentBeginOverlap`
  (params (OverlappedComponent :type "PrimitiveComponent Object Reference") (OtherActor :type "Actor Object Reference") (OtherComp :type "PrimitiveComponent Object Reference") (OtherBodyIndex :type Integer) (bFromSweep :type Boolean) (SweepResult :type "HitResult Structure (by ref)"))
  (bind _asbp_tower (cast `/Game/Blueprints/Blueprints/Tower/BP_Tower` OtherActor)
    (:`then`
      (if (not (== (`/Game/Blueprints/Blueprints/Tower/BP_Tower.ShootingRangeHibox` _asbp_tower) OtherComp))
        (if (not (`self.isPlaced?`)) :!label _label_2
          (`self.CantBePlaced`))))
    (:`CastFailed`
      (goto _label_2))))

(event `self.HitBox.OnComponentEndOverlap`
  (params (OverlappedComponent :type "PrimitiveComponent Object Reference") (OtherActor :type "Actor Object Reference") (OtherComp :type "PrimitiveComponent Object Reference") (OtherBodyIndex :type Integer))
  (if (`KismetArrayLibrary.Array_IsEmpty` (`PrimitiveComponent.GetOverlappingActors` (`self.HitBox`) null))
    (if (not (`self.isPlaced?`))
      (`self.CanBePlaced`))))

(fn `GetEnemy`
  (for _array_element (`PrimitiveComponent.GetOverlappingActors` (`self.ShootingRangeHibox`) "/Game/Blueprints/Blueprints/AI/Troops/BP_TroopsCharacter.BP_TroopsCharacter_C")
    (bind _asbp_troops_character (cast `/Game/Blueprints/Blueprints/AI/Troops/BP_TroopsCharacter` _array_element))
    (`KismetArrayLibrary.Array_AddUnique` (`self.Target`) _asbp_troops_character))
  (`self.Attack`))

(fn `PlaceTower`
  (set `self.isPlaced?` true)
  (`PrimitiveComponent.SetCollisionProfileName` (`self.HitBox`) "BlockAll" true)
  (`PrimitiveComponent.SetCollisionProfileName` (`self.ShootingRangeHibox`) "OverlapAll" true))

(fn `ProceduralAnimation`)

(fn `SetTowerMaterial`
  (params (Material :type "MaterialInterface Object Reference"))
  (`PrimitiveComponent.SetMaterial` (`self.basicTower1`) 0 Material))

(fn `TowerRadiusHitbox?`
  (params (Tower :type "/Game/Blueprints/Blueprints/Tower/BP_Tower Object Reference"))
  (if true
    _))

(fn `UserConstructionScript`
  (bind _returnvalue (`|GetDataTableRow` "/Game/Datatables/DT_TowerData.DT_TowerData" (`KismetStringLibrary.Conv_StringToName` (`KismetStringLibrary.Concat_StrStr` (`self.Name`) (`KismetStringLibrary.Conv_IntToString` (`self.Level`)))))
    (:`then`
      (`|ExecutionSequence`
        (:`then_0`
          (bind (_price _attackdamage _attackspeed _shootingrange) (break `/Game/Structs/S_TowerData` _returnvalue))
          (set `self.AttackDamage` _attackdamage))
        (:`then_1`
          (if (!= _attackspeed 0.0)
            (set `self.AttackSpeed` (/ 1.0 _attackspeed))))
        (:`then_2`
          (bind _output_get (set `self.ShootingRange` _shootingrange))
          (`SphereComponent.SetSphereRadius` (`self.ShootingRangeHibox`) _output_get true))))))