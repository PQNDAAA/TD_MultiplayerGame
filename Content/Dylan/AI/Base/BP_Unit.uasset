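; BP_Unit is a base unit Blueprint that tracks health in an SUnitInfo struct and displays it on a life bar.
; AnyDamage subtracts the damage from Health, without clamping or death handling, then refreshes the UI.
; UpdateUIBase, also called on BeginPlay, casts the Widget component's user widget to WBB_InfoBase and sets BarLife to the Health-to-MaxHealth ratio.
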(event `self.ReceiveBeginPlay`
  ;[1 1 1] Update UI at the beginning
  (`self.Update UI Base`))

(event `self.ReceiveAnyDamage`
  (params (Damage :type "Float (single-precision)") (DamageType :type "DamageType Object Reference") (InstigatedBy :type "Controller Object Reference") (DamageCauser :type "Actor Object Reference"))
  ;[1 1 1] Take Damage
  (`self.TakeDamage` Damage)
  (`self.Update UI Base`))

(fn `TakeDamage`
  (params (Damage :type "Float (double-precision)"))
  (locals (FinalHealth :type "Float (double-precision)"))
  (set `local.FinalHealth` (- (`.Health_11_2727ED6C4B492BC37991F5AD08FE0B56` (break `/Game/Struct/S_Unit` (`self.S_UnitInfo`))) Damage))
  ;[1 1 1] Set new var "Health"
  (`|VariableSetRef` (`.Health_11_2727ED6C4B492BC37991F5AD08FE0B56` (break `/Game/Struct/S_Unit` (`self.S_UnitInfo`))) (`local.FinalHealth`)))

(fn `Update UI Base`
  (bind (_name _damage _health _defense _speed _maxhealth) (break `/Game/Struct/S_Unit` (`self.S_UnitInfo`)))
  (bind _aswbb_info_base (cast `/Game/Widgets/GameMenu/Base/WBB_InfoBase` (`WidgetComponent.GetUserWidgetObject` (`self.Widget`))))
  (`ProgressBar.SetPercent` (`/Game/Widgets/GameMenu/Base/WBB_InfoBase.BarLife` _aswbb_info_base) (/ _health _maxhealth)))

(fn `UserConstructionScript`)