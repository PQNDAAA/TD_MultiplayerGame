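; Troop unit character that marches toward the base and deals repeated damage to actors it overlaps.
; Tick issues AI Move To toward the first base actor found, while BeginPlay fills the widget's life bar and name from the STroopsUnit struct.
; Overlap opens and enters a Gate that applies the struct's damage, prints it, then re-enters after a Delay, looping with nothing to close it.
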(event `self.ReceiveBeginPlay`
  ;[1 1 1] Update UI at the beginning
  (`self.UpdateUITroops`))

(event `self.ReceiveTick`
  (params (DeltaSeconds :type "Float (single-precision)"))
  ;[1 1 1] Move To The Base
  (`|AIMoveTo` self (0.0 0.0 0.0) (`self.GetBaseActor`)))

(event `self.ReceiveActorBeginOverlap`
  (params (OtherActor :type "Actor Object Reference"))
  (bind (_name _damage) (break `/Game/Struct/S_Unit` (`self.S_TroopsUnit`)))
  ;[1 1 1] Loop Damage when Collide
  (`|ExecutionSequence`
    (:`then_0`
      (goto _label :!via `Open`))
    (:`then_1`
      (`/Engine/EditorBlueprintResources/StandardMacros.Gate` true :!label _label
        (:`Exit`
          (bind _returnvalue (`GameplayStatics.ApplyDamage` OtherActor _damage null self))
          (`KismetSystemLibrary.PrintString` (`KismetTextLibrary.Conv_TextToString` (`|FormatText` "{Name}: {Damage}" _name _returnvalue)))
          (`KismetSystemLibrary.Delay` 5.0)
          (goto _label))))))

(fn `GetBaseActor`
  (returns (`Base Actor` :type "Actor Object Reference"))
  (bind _outactors (`GameplayStatics.GetAllActorsOfClass` (`self.Actor_Base`)))
  (return (`|GetArrayItem` _outactors)))

(fn `UpdateUITroops`
  (bind (_name _damage _health) (break `/Game/Struct/S_Unit` (`self.S_TroopsUnit`)))
  (bind _aswbb_troops_info (cast `/Game/Widgets/GameMenu/Troops/WBB_TroopsInfo` (`WidgetComponent.GetUserWidgetObject` (`self.Widget`))))
  (`ProgressBar.SetPercent` (`/Game/Widgets/GameMenu/Troops/WBB_TroopsInfo.BarLife` _aswbb_troops_info) _health)
  (`TextBlock.SetText` (`/Game/Widgets/GameMenu/Troops/WBB_TroopsInfo.TroopsName` _aswbb_troops_info) (`KismetTextLibrary.Conv_StringToText` _name)))

(fn `UserConstructionScript`)