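; BP_Banker is the banker's controllable camera, paired with a dedicated HUD.
; Axis inputs pan the Camera along its up and right vectors, with Shift raising the speed while held.
; The mouse wheel zooms along the forward vector, limited by checks on the camera's height.
; AddBankerUI creates the WBP_MainHUDBanker widget, switches to game-and-UI input and shows the cursor.
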(event `InputAxis|Move Forward / Backward`
  (params (AxisValue :type "Float (single-precision)"))
  (bind _camera (`self.Camera`))
  ;[1 1 1] Move Camera
  (`SceneComponent.K2_AddWorldOffset` _camera (* (`SceneComponent.GetUpVector` _camera) (* AxisValue (`self.CameraSpeed`))) false false))

(event `InputAxis|Move Right / Left`
  (params (AxisValue :type "Float (single-precision)"))
  (bind _camera (`self.Camera`))
  ;[1 1 1] Move Camera
  (`SceneComponent.K2_AddWorldOffset` _camera (* (`SceneComponent.GetRightVector` _camera) (* AxisValue (`self.CameraSpeed`))) false false))

(event `Key|MouseScrollUp`
  (params (Key :type "Key Structure"))
  (bind _camera (`self.Camera`))
  (bind (_returnvalue_x _returnvalue_y _returnvalue_z) (`KismetMathLibrary.BreakVector` (`SceneComponent.K2_GetComponentLocation` _camera)))
  ;[1 1 1] Zoom / Dezoom Camera
  (:`Pressed`
    (if (> _returnvalue_z (`self.CameraZoomMax`))
      (`SceneComponent.K2_AddWorldOffset` _camera (* (`SceneComponent.GetForwardVector` _camera) (`self.CameraZoomSpeed`)) false false))))

(event `InputAction|Shift`
  (params (Key :type "Key Structure"))
  ;[1 1 1] Increase Camera Speed
  (:`Pressed`
    (set `self.CameraSpeed` 10.0))
  (:`Released`
    (set `self.CameraSpeed` 5.0)))

(event `Key|MouseScrollDown`
  (params (Key :type "Key Structure"))
  (bind _camera (`self.Camera`))
  (bind (_returnvalue_x _returnvalue_y _returnvalue_z) (`KismetMathLibrary.BreakVector` (`SceneComponent.K2_GetComponentLocation` _camera)))
  ;[1 1 1] Zoom / Dezoom Camera
  (:`Pressed`
    (if (< _returnvalue_z (`self.CameraZoomMin`))
      (`SceneComponent.K2_AddWorldOffset` _camera (* (* (`SceneComponent.GetForwardVector` _camera) -1) (`self.CameraZoomSpeed`)) false false))))

(event `AddBankerUI`
  (bind _returnvalue (`GameplayStatics.GetPlayerController` 0))
  ;[1 1 1] Add UI
  (bind _returnvalue_2 (`|CreateWidget` "/Game/Widgets/GameMenu/Banker/WBP_MainHUDBanker.WBP_MainHUDBanker_C"))
  (`UserWidget.AddToViewport` _returnvalue_2 0)
  (`WidgetBlueprintLibrary.SetInputMode_GameAndUIEx` _returnvalue null "DoNotLock" false)
  (set `PlayerController.bShowMouseCursor` true _returnvalue))

(fn `UserConstructionScript`
  (`parent.UserConstructionScript`))