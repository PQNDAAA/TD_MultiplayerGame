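; Player controller that lets the local player pick a class, banker or not, when the Game level starts.
; On BeginPlay it shows the WBP_ChooseClass widget with UI-only input.
; CreatePlayer_Server forwards the IsBanker choice to BP_ThirdPersonGameMode, which spawns the player for this controller and then runs SpawnSpeed.
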(event `self.ReceiveBeginPlay`
  (bind _returnvalue (`GameplayStatics.GetCurrentLevelName` true))
  (if (`KismetStringLibrary.EqualEqual_StrStr` _returnvalue "Game")
    (if (`self.IsLocalPlayerController`)
      (`self.ChooseClass`))))

(event `CreatePlayer_Server`
  (params (`isBanker?` :type Boolean))
  (bind _asbp_third_person_game_mode (cast `/Game/Blueprint/BP_ThirdPersonGameMode` (`GameplayStatics.GetGameMode`)))
  (`/Game/Blueprint/BP_ThirdPersonGameMode.Spawn Player` _asbp_third_person_game_mode self `isBanker?`)
  (`/Game/Blueprint/BP_ThirdPersonGameMode.Spawn Speed` _asbp_third_person_game_mode))

(event `ChooseClass`
  (bind _returnvalue (`|CreateWidget` "/Game/Widgets/MainMenu/WBP_ChooseClass.WBP_ChooseClass_C" self))
  (`UserWidget.AddToViewport` _returnvalue 0)
  (`WidgetBlueprintLibrary.SetInputMode_UIOnlyEx` self null))

(fn `UserConstructionScript`)